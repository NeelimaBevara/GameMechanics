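; Slot machine Blueprint that charges the interacting character 50 from their balance and animates a spin, provided they can afford it.
; The interact event deducts the cost, then a sequence starts timelines that drive the roll rotation of the lever and three wheels.
; Each wheel starts after its own random delay to stagger the spin, while the lever moves at once.
; The graph contains no outcome or payout logic.
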(event `/Game/Blueprints/Interfaces/BPI_Interact.InteractEvent`
  (params (CharacterRef :type "Character Object Reference"))
  (bind _money (message `/Game/Blueprints/Interfaces/BPI_Character.GetCurrentBalance` CharacterRef))
  (if (>= _money 50)
    (message `/Game/Blueprints/Interfaces/BPI_Character.UpdateBalance` CharacterRef (- _money 50))
    (`|ExecutionSequence`
      (:`then_0`
        (bind (_direction _newtrack_0) (`Timeline|MoveHandle` :!via `PlayFromStart`)
          (:`Update`
            (`SceneComponent.K2_SetRelativeRotation` (`self.JackpotLever`) (`KismetMathLibrary.MakeRotator` _newtrack_0) false false))))
      (:`then_1`
        (`KismetSystemLibrary.Delay` (`KismetMathLibrary.RandomFloatInRange` 0.0 0.9))
        (bind (_direction_2 _newtrack_0_2) (`Timeline|Timeline` :!via `PlayFromStart`)
          (:`Update`
            (`SceneComponent.K2_SetRelativeRotation` (`self.Wheel01`) (`KismetMathLibrary.MakeRotator` _newtrack_0_2) false false))))
      (:`then_2`
        (`KismetSystemLibrary.Delay` (`KismetMathLibrary.RandomFloatInRange` 0.0 0.5))
        (bind (_direction_3 _newtrack_0_3) (`Timeline|Timeline_0` :!via `PlayFromStart`)
          (:`Update`
            (`SceneComponent.K2_SetRelativeRotation` (`self.Wheel02`) (`KismetMathLibrary.MakeRotator` _newtrack_0_3) false false))))
      (:`then_3`
        (`KismetSystemLibrary.Delay` (`KismetMathLibrary.RandomFloatInRange` 0.4 1.2))
        (bind (_direction_4 _newtrack_0_4) (`Timeline|Timeline_1` :!via `PlayFromStart`)
          (:`Update`
            (`SceneComponent.K2_SetRelativeRotation` (`self.Wheel03`) (`KismetMathLibrary.MakeRotator` _newtrack_0_4) false false)))))))

(fn `UserConstructionScript`)